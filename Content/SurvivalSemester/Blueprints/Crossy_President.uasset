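; Crossy club president NPC in Survival Semester that shows dialogue when the third-person player character enters its trigger box.
; It creates a dialogue widget on BeginPlay and picks the line from its own world X position: a club invitation or a congratulatory send-back message, so one Blueprint covers both cases.
; Overlap adds the widget and shows the mouse cursor; leaving removes and hides them.
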(event OnComponentBeginOverlap(Box)
  (params (OverlappedComponent :type Primitive%20Component%20Object%20Reference) (OtherActor :type Actor%20Object%20Reference) (OtherComp :type Primitive%20Component%20Object%20Reference) (OtherBodyIndex :type Integer) (bFromSweep :type Boolean) (SweepResult :type Hit%20Result%20Structure%20%28by%20ref%29))
  (bind _dialogue (Variables|Default|GetDialogue))
  (bind _crpresidentdialogue (Variables|/Game/SurvivalSemester/Blueprints/Crossy_President_Dialogue.Crossy_President_Dialogue_C|GetCRPresidentDialogue _dialogue))
  (bind _asbp_third_person_character (Utilities|Casting|CastToBP_ThirdPersonCharacter OtherActor))
  (if (<= (.x (.location (Transformation|GetActorTransform))) 5e+03)
    (Rendering|Components|TextRender|SetText _crpresidentdialogue "Wanna join the crossy club?")
    (else
      (Rendering|Components|TextRender|SetText _crpresidentdialogue "Congrats! I'll send you back now.")))
  (UserInterface|Viewport|AddtoViewport _dialogue 0)
  (Variables|/Script/Engine.PlayerController|SetbShowMouseCursor (Game|GetPlayerController (Variables|/Script/Engine.Pawn|GetPlayerState _asbp_third_person_character)) true))

(event OnComponentEndOverlap(Box)
  (params (OverlappedComponent :type Primitive%20Component%20Object%20Reference) (OtherActor :type Actor%20Object%20Reference) (OtherComp :type Primitive%20Component%20Object%20Reference) (OtherBodyIndex :type Integer))
  (bind _asbp_third_person_character (Utilities|Casting|CastToBP_ThirdPersonCharacter OtherActor))
  (Widget|RemovefromParent (Variables|Default|GetDialogue))
  (Variables|/Script/Engine.PlayerController|SetbShowMouseCursor (Game|GetPlayerController (Variables|/Script/Engine.Pawn|GetPlayerState _asbp_third_person_character)) false))

(event EventBeginPlay
  (bind _returnvalue (UserInterface|CreateWidget "/Game/SurvivalSemester/Blueprints/Crossy_President_Dialogue.Crossy_President_Dialogue_C" (Game|GetPlayerController 0)))
  (Variables|Default|SetDialogue _returnvalue))

(fn ConstructionScript)