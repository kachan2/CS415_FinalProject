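; Ballz is a hazard ball actor that knocks the player back and tallies hits in the Survival Semester game.
; On sphere overlap with the third-person character, it teleports that character to a fixed location, then increments the Running_President's BallsTakenWidget score and refreshes its text.
; Each tick it destroys itself once its world X position drops to or below a fixed threshold.
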(event OnComponentBeginOverlap(Sphere)
  (params (OverlappedComponent :type Primitive%20Component%20Object%20Reference) (OtherActor :type Actor%20Object%20Reference) (OtherComp :type Primitive%20Component%20Object%20Reference) (OtherBodyIndex :type Integer) (bFromSweep :type Boolean) (SweepResult :type Hit%20Result%20Structure%20%28by%20ref%29))
  (bind _asbp_third_person_character (Utilities|Casting|CastToBP_ThirdPersonCharacter OtherActor))
  (Transformation|SetActorTransform _asbp_third_person_character (Math|Transform|MakeTransform "5400.000000,4500.000000,1600.000000" "0, 0, 0" "1.000000,1.000000,1.000000"))
  (bind _returnvalue (Actor|GetActorOfClass "/Game/SurvivalSemester/Blueprints/Running_President.Running_President_C"))
  (bind _result (Math|Integer|IncrementInt (Variables|/Game/SurvivalSemester/Blueprints/Ballz_Taken.Ballz_Taken_C|GetScore_Num (Variables|/Game/SurvivalSemester/Blueprints/Running_President.Running_President_C|GetBallsTakenWidget _returnvalue)))
    (:%20%20
      (Variables|/Game/SurvivalSemester/Blueprints/Ballz_Taken.Ballz_Taken_C|SetScore_Num (Variables|/Game/SurvivalSemester/Blueprints/Running_President.Running_President_C|GetBallsTakenWidget _returnvalue) _result)
      (Rendering|Components|TextRender|SetText (Variables|/Game/SurvivalSemester/Blueprints/Ballz_Taken.Ballz_Taken_C|GetScore (Variables|/Game/SurvivalSemester/Blueprints/Running_President.Running_President_C|GetBallsTakenWidget _returnvalue)) (Utilities|Text|ToText(Integer) _result)))))

(event EventTick
  (params (DeltaSeconds :type Float%20%28single-precision%29))
  (if (<= (.x (.location (Transformation|GetActorTransform))) 5.6e+03)
    (Actor|DestroyActor)))

(fn ConstructionScript)