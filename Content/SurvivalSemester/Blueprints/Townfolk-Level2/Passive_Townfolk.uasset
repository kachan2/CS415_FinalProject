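; Passive townfolk AI character for Level 2 that flees the player when hurt instead of fighting back.
; AnyDamage, gated by an IsDamaged flag, turns it relative to the damage causer, applies knockback and decrements health, then either runs away or dies.
; RunAway uses AI MoveTo toward a point directly away from the player, then calls Roam whether the move succeeds or fails.
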(event Custom|RunAway
  (bind _returnvalue (Transformation|GetActorLocation))
  (bind _returnvalue_2 (Game|GetPlayerCharacter 0))
  (bind _returnvalue_3 (Transformation|GetActorLocation _returnvalue_2))
  (bind _returnvalue_4 (Math|Rotator|FindLookatRotation _returnvalue _returnvalue_3))
  (bind _returnvalue_5 (Math|Vector|GetForwardVector _returnvalue_4))
  (bind _returnvalue_6 (* _returnvalue_5 -5e+02))
  (bind _returnvalue_7 (+ _returnvalue_6 _returnvalue))
  (AI|AIMoveTo self (Math|Vector|MakeVector (.x _returnvalue_7) (.y _returnvalue_7) (.z _returnvalue_7)) 0 5.0 false
    (:OnSuccess
      _)
    (:OnFail
      _))
  (CallFunction|Roam))

(event EventBeginPlay
  (|CallParentFunction) ; This node is disabled and will not be called.\nDrag off pins to build functionality.
)

(event Collision|EventActorBeginOverlap
  (params (OtherActor :type Actor%20Object%20Reference))
  (|CallParentFunction OtherActor) ; This node is disabled and will not be called.\nDrag off pins to build functionality.
)

(event EventTick
  (params (DeltaSeconds :type Float%20%28single-precision%29))
  (|CallParentFunction DeltaSeconds) ; This node is disabled and will not be called.\nDrag off pins to build functionality.
)

(event Game|Damage|EventAnyDamage
  (params (Damage :type Float%20%28single-precision%29) (DamageType :type Damage%20Type%20Object%20Reference) (InstigatedBy :type Controller%20Object%20Reference) (DamageCauser :type Actor%20Object%20Reference))
  (if (not (Variables|Default|GetIsDamaged))
    (Variables|Default|SetIsDamaged true)
    (CallFunction|Rotate DamageCauser)
    (CallFunction|Knockback)
    (bind _isalive (CallFunction|DecrementHealth Damage))
    (if _isalive
      (Variables|Default|SetIsDamaged false)
      (CallFunction|RunAway)
      (else
        (CallFunction|Death)))))

(fn ConstructionScript
  (|CallParentFunction))