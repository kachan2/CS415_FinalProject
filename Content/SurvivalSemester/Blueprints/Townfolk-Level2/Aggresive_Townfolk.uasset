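; Aggressive townfolk NPC for Level 2 that retaliates against the player when damaged.
; A hit triggers rotation, knockback and a health decrement, then either death or, after a brief invulnerability delay, a five-round attack loop.
; Each round moves to the player and attacks whether or not the move succeeds, opening a timed window where capsule overlaps deal LightAttack damage with a negative value.
; When the rounds run out, it returns to roaming.
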(event OnComponentBeginOverlap(CapsuleComponent)
  (params (OverlappedComponent :type Primitive%20Component%20Object%20Reference) (OtherActor :type Actor%20Object%20Reference) (OtherComp :type Primitive%20Component%20Object%20Reference) (OtherBodyIndex :type Integer) (bFromSweep :type Boolean) (SweepResult :type Hit%20Result%20Structure%20%28by%20ref%29))
  (if (Variables|Default|GetDamageActivate)
    (Game|Damage|ApplyDamage OtherActor -1e+01 0 self "/Game/SurvivalSemester/Blueprints/Bosses/LightAttack.LightAttack_C")))

(event Custom|Attack
  (bind _attackex (Variables|Default|GetAttackEx))
  (if (> (Variables|Default|GetCounter) 0)
    (AI|AIMoveTo self "0, 0, 0" (Game|GetPlayerCharacter 0) 5.0 false
      (:OnSuccess
        _)
      (:OnFail
        _))
    (Utilities|FlowControl|Delay 1.0)
    (Variables|Default|SetDamageActivate true)
    (Variables|/Game/SurvivalSemester/Blueprints/AttackExclaimer.AttackExclaimer_C|SetWillAttack? _attackex true)
    (Utilities|FlowControl|Delay 2.0)
    (Variables|/Game/SurvivalSemester/Blueprints/AttackExclaimer.AttackExclaimer_C|SetWillAttack? _attackex false)
    (Variables|Default|SetDamageActivate false)
    (Variables|Default|SetCounter (- (Variables|Default|GetCounter) 1))
    (CallFunction|Attack)
    (else
      (CallFunction|Roam))))

(event EventBeginPlay)

(event Collision|EventActorBeginOverlap
  (params (OtherActor :type Actor%20Object%20Reference)))

(event EventTick
  (params (DeltaSeconds :type Float%20%28single-precision%29)))

(event Game|Damage|EventAnyDamage
  (params (Damage :type Float%20%28single-precision%29) (DamageType :type Damage%20Type%20Object%20Reference) (InstigatedBy :type Controller%20Object%20Reference) (DamageCauser :type Actor%20Object%20Reference))
  (if (not (Variables|Default|GetIsDamaged))
    (Variables|Default|SetIsDamaged true)
    (CallFunction|Rotate DamageCauser)
    (CallFunction|Knockback)
    (bind _isalive (CallFunction|DecrementHealth Damage))
    (if _isalive
      (Utilities|FlowControl|Delay 2.0)
      (Variables|Default|SetIsDamaged false)
      (Variables|Default|SetCounter 5)
      (CallFunction|Attack)
      (else
        (CallFunction|Death)))))

(fn ConstructionScript)