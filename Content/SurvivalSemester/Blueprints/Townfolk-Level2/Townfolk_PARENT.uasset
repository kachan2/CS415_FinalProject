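; Parent character for Level 2 townfolk NPCs that wander, take damage and drop money on death.
; Roam loops random reachable-point moves with random pauses, while Tick turns the floating health bar and attack indicator toward the camera.
; DecrementHealth adds a delta to health, updates the bar and returns whether health remains.
; Death, Rotate and Knockback events handle delayed destruction with a BP_Money spawn, turning toward a target and backward launches.
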(event Custom|Roam
  ;[1 1 1] Roam
  (AI|AIMoveTo self (.RandomLocation (AI|Navigation|GetRandomReachablePointinRadius (Transformation|GetActorLocation) 1e+03 0 0)) 0 5.0 false
    (:then
      (Utilities|FlowControl|Delay (Math|Random|RandomFloatinRange 0.0 8.0))
      (CallFunction|Roam))))

(event Custom|Rotate
  (params (TargetToLookAt :type Actor%20Object%20Reference))
  ;[1 1 1] Rotate
  (Transformation|SetActorRotation (Math|Interpolation|RInterpTo (Transformation|GetActorRotation) (Math|Rotator|FindLookatRotation (Transformation|GetActorLocation) (Transformation|GetActorLocation TargetToLookAt)) (Utilities|Time|GetWorldDeltaSeconds) 0.0)))

(event Custom|Knockback
  ;[1 1 1] Knockback
  (Character|LaunchCharacter (* (Math|Vector|GetForwardVector (Variables|Default|GetScene)) -2e+03) false false)
  (Utilities|FlowControl|Delay 1.5))

(event Custom|Death
  (bind _returnvalue (Transformation|GetActorLocation))
  ;[1 1 1] Death
  (Pawn|Components|CharacterMovement|DisableMovement (Variables|Character|GetCharacterMovement))
  (Utilities|FlowControl|Delay 2.0)
  (Game|SpawnActorfromClass "/Game/SurvivalSemester/Inventory/Bluprints/BP_Money.BP_Money_C" (Math|Transform|MakeTransform (Math|Vector|MakeVector (.x _returnvalue) (.y _returnvalue) 0.0) "0, 0, 0" "1.000000,1.000000,1.000000") "AdjustIfPossibleButAlwaysSpawn" "MultiplyWithRoot" 0 0)
  (Actor|DestroyActor))

(event EventBeginPlay
  (bind _currenthealth (Variables|Default|GetCurrentHealth))
  ;[1 1 1] Initialize
  (Variables|/Script/Engine.CharacterMovementComponent|SetMaxWalkSpeed (Variables|Character|GetCharacterMovement) 315.0)
  (bind _asfloating_health_bar (Utilities|Casting|CastToFloatingHealthBar (UserInterface|GetUserWidgetObject (Variables|Default|GetFloatingHealthBar))))
  (bind _output_get (Variables|Default|SetFloatingHB _asfloating_health_bar))
  (Variables|/Game/SurvivalSemester/Blueprints/FloatingHealthBar.FloatingHealthBar_C|SetCurrHealth _output_get _currenthealth)
  (Variables|/Game/SurvivalSemester/Blueprints/FloatingHealthBar.FloatingHealthBar_C|SetMaxHealth _output_get _currenthealth)
  (bind _asattack_exclaimer (Utilities|Casting|CastToAttackExclaimer (UserInterface|GetUserWidgetObject (Variables|Default|GetAttackIndicator))))
  (bind _output_get_2 (Variables|Default|SetAttackEx _asattack_exclaimer))
  (Variables|/Game/SurvivalSemester/Blueprints/AttackExclaimer.AttackExclaimer_C|SetWillAttack? _output_get_2 false)
  (CallFunction|Roam))

(event Collision|EventActorBeginOverlap
  (params (OtherActor :type Actor%20Object%20Reference)))

(event EventTick
  (params (DeltaSeconds :type Float%20%28single-precision%29))
  (bind _returnvalue (Game|GetPlayerCameraManager 0))
  (bind _floatinghealthbar (Variables|Default|GetFloatingHealthBar))
  (bind _attackindicator (Variables|Default|GetAttackIndicator))
  (bind _rootcomponent (Variables|/Script/Engine.Actor|GetRootComponent _returnvalue))
  (bind _returnvalue_2 (Transformation|GetWorldLocation _rootcomponent))
  (Transformation|SetWorldRotation _floatinghealthbar (Math|Rotator|FindLookatRotation (Transformation|GetWorldLocation _floatinghealthbar) _returnvalue_2) false false)
  (Transformation|SetWorldRotation _attackindicator (Math|Rotator|FindLookatRotation (Transformation|GetWorldLocation _attackindicator) _returnvalue_2) false false))

(fn ConstructionScript)

(fn DecrementHealth
  (params (DecrementHealth :type Float%20%28double-precision%29))
  (bind _output_get (Variables|Default|SetCurrentHealth (+ (Variables|Default|GetCurrentHealth) DecrementHealth)))
  (bind _output_get_2 (Variables|/Game/SurvivalSemester/Blueprints/FloatingHealthBar.FloatingHealthBar_C|SetCurrHealth (Variables|Default|GetFloatingHB) _output_get))
  (return (> _output_get_2 0.0)))