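; Moving platform actor that shuttles back and forth along the world Y axis between StartPos and EndPos.
; BeginPlay gives each instance a random speed and a random initial direction.
; Tick offsets the actor's Y location by that speed and flips direction once a bound is reached.
; Movement is a fixed step per frame without delta time, so its pace depends on frame rate.
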(event EventBeginPlay
  (Variables|Default|SetSpeed (* (+ (Math|Random|RandomFloat) 0.3) 2e+01))
  (Variables|Default|SetRight? (<= (Math|Random|RandomFloat) 0.5)))

(event EventTick
  (params (DeltaSeconds :type Float%20%28single-precision%29))
  (bind _returnvalue (Transformation|GetActorTransform))
  (bind _returnvalue_2 (Transformation|GetActorTransform))
  (if (Variables|Default|GetRight?)
    (if (>= (.y (.location _returnvalue_2)) (Variables|Default|GetEndPos))
      (Variables|Default|SetRight? false)
      (else
        (Transformation|SetActorTransform (Math|Transform|MakeTransform (Math|Vector|MakeVector (.x (.location _returnvalue_2)) (+ (.y (.location _returnvalue_2)) (Variables|Default|GetSpeed)) (.z (.location _returnvalue_2))) "0, 0, 0" "1.000000,1.000000,1.000000"))))
    (elif (<= (.y (.location _returnvalue)) (Variables|Default|GetStartPos))
      (Variables|Default|SetRight? true)
      (else
        (Transformation|SetActorTransform (Math|Transform|MakeTransform (Math|Vector|MakeVector (.x (.location _returnvalue)) (- (.y (.location _returnvalue)) (Variables|Default|GetSpeed)) (.z (.location _returnvalue))) "0, 0, 0" "1.000000,1.000000,1.000000"))))))

(fn ConstructionScript)