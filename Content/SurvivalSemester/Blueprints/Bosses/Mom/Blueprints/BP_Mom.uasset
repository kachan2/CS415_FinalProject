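; BP_Mom is the Mom boss, an AI pawn that wanders at random and watches for the player.
; From BeginPlay, a self-calling Roam event issues AI MoveTo to a random reachable point nearby, then repeats after a short delay.
; A PawnSensing sighting sets IsSeeingPlayer but does not stop roaming; the minigame it announces is only a debug print.
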(event OnSeePawn(PawnSensing)
  (params (Pawn :type Pawn%20Object%20Reference))
  (Variables|Default|SetIsSeeingPlayer? true)
  (Development|PrintString "spotted. load minigame"))

(event Custom|Roam
  (AI|AIMoveTo self (.RandomLocation (AI|Navigation|GetRandomReachablePointinRadius (Transformation|GetActorLocation) 4e+02 0 0)) 0 5.0 false
    (:then
      (Utilities|FlowControl|Delay 1.0)
      (CallFunction|Roam))))

(event EventBeginPlay
  (CallFunction|Roam))

(fn ConstructionScript)