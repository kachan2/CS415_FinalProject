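; Bully boss enemy that roams to random nearby points until PawnSensing spots a pawn or it takes damage, then chases the player.
; On reaching the player it plays a random punch or rarer kick; sphere overlaps deal damage only while the matching peak flag is set.
; Damage values are negative and added to health, triggering a hit reaction or a stunned death before destruction.
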(event OnSeePawn(PawnSensing)
  (params (Pawn :type Pawn%20Object%20Reference))
  ;[1 1 1] Initiate Chase
  (if (not (Variables|Default|GetIsDead))
    (Variables|Default|SetIsRoaming false)
    (Variables|Default|SetSeesPlayer? true)
    (Variables|/Script/Engine.CharacterMovementComponent|SetMaxWalkSpeed (Variables|Character|GetCharacterMovement) 6e+02)
    (CallFunction|Chase)))

(event OnComponentBeginOverlap(Sphere)
  (params (OverlappedComponent :type Primitive%20Component%20Object%20Reference) (OtherActor :type Actor%20Object%20Reference) (OtherComp :type Primitive%20Component%20Object%20Reference) (OtherBodyIndex :type Integer) (bFromSweep :type Boolean) (SweepResult :type Hit%20Result%20Structure%20%28by%20ref%29))
  ;[1 1 1] Logic for Bully Light Attack
  (if (Variables|Default|GetPunchPeak)
    (Development|PrintString "PunchTime")
    (bind _asbp_third_person_character (Utilities|Casting|CastToBP_ThirdPersonCharacter OtherActor))
    (Game|Damage|ApplyDamage _asbp_third_person_character -1e+01 0 self "/Game/SurvivalSemester/Blueprints/Bosses/LightAttack.LightAttack_C")))

(event OnComponentBeginOverlap(KickSphere_0)
  (params (OverlappedComponent :type Primitive%20Component%20Object%20Reference) (OtherActor :type Actor%20Object%20Reference) (OtherComp :type Primitive%20Component%20Object%20Reference) (OtherBodyIndex :type Integer) (bFromSweep :type Boolean) (SweepResult :type Hit%20Result%20Structure%20%28by%20ref%29))
  ;[1 1 1] Kicking
  (if (Variables|Default|GetKickPeak)
    (bind _asbp_third_person_character (Utilities|Casting|CastToBP_ThirdPersonCharacter OtherActor))
    (Game|Damage|ApplyDamage _asbp_third_person_character -15.0 0 self "/Game/SurvivalSemester/Blueprints/Bosses/HeavyAttack.HeavyAttack_C")))

(event Custom|Roam
  ;[1 1 1] Roaming Logic
  (Variables|Default|SetIsRoaming true)
  (Variables|/Script/Engine.CharacterMovementComponent|SetMaxWalkSpeed (Variables|Character|GetCharacterMovement) 315.0)
  (AI|AIMoveTo self (.RandomLocation (AI|Navigation|GetRandomReachablePointinRadius (Transformation|GetActorLocation) 1e+03 0 0)) 0 5.0 false
    (:then
      (Utilities|FlowControl|Delay 5.0)
      (CallFunction|Roam))))

(event Custom|Chase
  ;[1 1 1] Chasing Logic
  (AI|AIMoveTo self "0, 0, 0" (Game|GetPlayerCharacter 0) 0.0 true
    (:OnSuccess
      (CallFunction|Attack)
      (CallFunction|Chase))))

(event Custom|Death
  ;[1 1 1] Death
  (Variables|Default|SetIsDead true)
  (Variables|/Script/AIModule.PawnSensingComponent|SetSightRadius (Variables|Default|GetPawnSensing) 0.0)
  (Pawn|Components|CharacterMovement|DisableMovement (Variables|Character|GetCharacterMovement))
  (Components|Animation|PlayAnimation (Variables|Character|GetMesh) "/Game/SurvivalSemester/Blueprints/Bosses/Animation/Stunned.Stunned" false)
  (Utilities|FlowControl|Delay 5.0)
  (Actor|DestroyActor))

(event Custom|Attack
  ;[1 1 1] Attacking Logic
  (CallFunction|Rotate (Game|Player|GetPlayerPawn 0))
  (Pawn|Components|CharacterMovement|DisableMovement (Variables|Character|GetCharacterMovement))
  (if (Variables|Default|GetCanAttack)
    (if (not (Variables|Default|GetIsDamaged))
      (Variables|Default|SetCanAttack false)
      (switch int (Math|Random|RandomInteger 5)
        (:Default
          ;;[1 1 1] Light Attack (Punch)
          (Components|Animation|PlayAnimation (Variables|Character|GetMesh) "/Game/SurvivalSemester/Blueprints/Bosses/Animation/Punching_Slow.Punching_Slow" false)
          (Utilities|FlowControl|Delay 1.5))
        (:0
          ;;[1 1 1] Heavy Attack (Kick)
          (Components|Animation|PlayAnimation (Variables|Character|GetMesh) "/Game/SurvivalSemester/Blueprints/Bosses/Animation/Mma_Kick_Slow_.Mma_Kick_Slow_" false)
          (Utilities|FlowControl|Delay 3.0)))
      (Pawn|Components|CharacterMovement|SetMovementMode (Variables|Character|GetCharacterMovement) "MOVE_Walking" 0)
      ;;[1 1 1] Reset Attack for Bully
      (Variables|Default|SetCanAttack true)
      (Components|Animation|SetAnimationMode (Variables|Character|GetMesh) "AnimationBlueprint" true)
      (Variables|/Script/Engine.CharacterMovementComponent|SetMaxWalkSpeed (Variables|Character|GetCharacterMovement) 6e+02))))

(event Custom|PauseAnims
  (bind _mesh (Variables|Character|GetMesh))
  ;[1 1 1] PauseAnimations
  (Variables|/Script/Engine.SkeletalMeshComponent|SetbPauseAnims _mesh true)
  (Variables|/Script/Engine.SkeletalMeshComponent|SetbNoSkeletonUpdate _mesh true))

(event Custom|Rotate
  (params (TargettoLookAt :type Actor%20Object%20Reference))
  ;[1 1 1] Rotation
  (Transformation|SetActorRotation (Math|Interpolation|RInterpTo (Transformation|GetActorRotation) (Math|Rotator|FindLookatRotation (Transformation|GetActorLocation) (Transformation|GetActorLocation TargettoLookAt)) (Utilities|Time|GetWorldDeltaSeconds) 0.0)))

(event EventBeginPlay
  ;[1 1 1] Initalization
  (Variables|/Script/Engine.CharacterMovementComponent|SetMaxWalkSpeed (Variables|Character|GetCharacterMovement) 315.0)
  (CallFunction|Roam))

(event Game|Damage|EventAnyDamage
  (params (Damage :type Float%20%28single-precision%29) (DamageType :type Damage%20Type%20Object%20Reference) (InstigatedBy :type Controller%20Object%20Reference) (DamageCauser :type Actor%20Object%20Reference))
  ;[1 1 1] Damage
  (CallFunction|Rotate DamageCauser)
  (if (not (Variables|Default|GetIsDamaged))
    ;;[1 1 1] Apply damage, set damage animation
    (Variables|Default|SetIsDamaged true)
    (bind _output_get (Variables|Default|SetHealthBar (+ (Variables|Default|GetHealthBar) Damage)))
    (Development|PrintString (Utilities|String|ToString(Float) _output_get))
    (if (> (Variables|Default|GetHealthBar) 0.0)
      (Components|Animation|PlayAnimation (Variables|Character|GetMesh) "/Game/SurvivalSemester/Blueprints/Bosses/Animation/Head_Hit_Slow.Head_Hit_Slow" false)
      (Utilities|FlowControl|Delay 2.0)
      (Components|Animation|SetAnimationMode (Variables|Character|GetMesh) "AnimationBlueprint" true)
      ;;[1 1 1] Did the player sneak up on the bully?
      (Variables|Default|SetIsRoaming false)
      (Variables|Default|SetSeesPlayer? true)
      (Variables|/Script/Engine.CharacterMovementComponent|SetMaxWalkSpeed (Variables|Character|GetCharacterMovement) 6e+02)
      (Variables|Default|SetIsDamaged false)
      (Pawn|Components|CharacterMovement|SetMovementMode (Variables|Character|GetCharacterMovement) "MOVE_Walking" 0)
      (CallFunction|Chase)
      (else
        (CallFunction|Death)))))

(event Input|KeyboardEvents|DebugKeyK
  (params (Key :type Key%20Structure :default "None") (ActionValue :type Input%20Action%20Value%20Structure))
  (:Pressed
    (CallFunction|Death)))

(fn ConstructionScript)