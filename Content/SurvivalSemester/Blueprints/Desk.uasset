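; Desk is an interactable actor in Survival Semester that may offer a dialogue to the third-person player.
; On BeginPlay it creates its Desk_Dialogue widget and randomly marks itself active, roughly a one-in-five chance.
; When the player character overlaps an active desk, it shows the dialogue and mouse cursor, then hides both when the overlap ends.
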(event EventBeginPlay
  (bind _returnvalue (UserInterface|CreateWidget "/Game/SurvivalSemester/Blueprints/Desk_Dialogue.Desk_Dialogue_C"))
  (Variables|Default|SetDialogue _returnvalue)
  (if (<= (Math|Random|RandomFloat) 0.2)
    (Variables|Default|SetActive true)
    (else
      (Variables|Default|SetActive false))))

(event Collision|EventActorBeginOverlap
  (params (OtherActor :type Actor%20Object%20Reference))
  (bind _asbp_third_person_character (Utilities|Casting|CastToBP_ThirdPersonCharacter OtherActor))
  (if (Variables|Default|GetActive)
    (UserInterface|Viewport|AddtoViewport (Variables|Default|GetDialogue) 0)
    (Variables|/Script/Engine.PlayerController|SetbShowMouseCursor (Game|GetPlayerController (Variables|/Script/Engine.Pawn|GetPlayerState _asbp_third_person_character)) true)))

(event Collision|EventActorEndOverlap
  (params (OtherActor :type Actor%20Object%20Reference))
  (Utilities|Casting|CastToBP_ThirdPersonCharacter OtherActor)
  (if (Variables|Default|GetActive)
    (Widget|RemovefromParent (Variables|Default|GetDialogue))
    (Variables|/Script/Engine.PlayerController|SetbShowMouseCursor (Game|GetPlayerController (Variables|/Script/Engine.Pawn|GetPlayerState (stale Collision|EventActorBeginOverlap _asbp_third_person_character))) false)))

(fn ConstructionScript)