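; Shooter actor that randomly spawns Ballz projectiles at its own transform and drives their movement.
; Tick counts frames, then past a threshold rolls a chance each frame, resetting the counter after a spawn.
; Every frame it also shifts all Ballz in the world along negative X, independent of delta time.
; A separate SpawnBallz function spawns one at an offset but is not called here.
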(event EventBeginPlay)

(event Collision|EventActorBeginOverlap
  (params (OtherActor :type Actor%20Object%20Reference)))

(event EventTick
  (params (DeltaSeconds :type Float%20%28single-precision%29))
  (bind _result (Math|Integer|IncrementInt (Variables|Default|GetTimer))
    (:%20%20
      (bind _output_get (Variables|Default|SetTimer _result))
      (if (>= _output_get 25)
        (if (<= (Math|Random|RandomFloat) 0.2)
          (Game|SpawnActorfromClass "/Game/SurvivalSemester/Blueprints/Ballz.Ballz_C" (Transformation|GetActorTransform) "Undefined" "MultiplyWithRoot" 0 0)
          (Variables|Default|SetTimer 0)))
      (bind _outactors (Actor|GetAllActorsOfClass "/Game/SurvivalSemester/Blueprints/Ballz.Ballz_C"))
      (for _array_element _outactors
        (Transformation|SetActorTransform _array_element (Math|Transform|MakeTransform (+ (.location (Transformation|GetActorTransform _array_element)) "-5.000000,0.000000,0.000000") "0, 0, 0" "1.000000,1.000000,1.000000"))))))

(fn ConstructionScript)

(fn SpawnBallz
  (Game|SpawnActorfromClass "/Game/SurvivalSemester/Blueprints/Ballz.Ballz_C" (Math|Transform|MakeTransform (+ (.location (Transformation|GetActorTransform)) "-100.000000,0.000000,0.000000") "0, 0, 0" "1.000000,1.000000,1.000000") "Undefined" "MultiplyWithRoot" 0 0))