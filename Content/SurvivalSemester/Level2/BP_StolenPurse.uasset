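; Level 2 dialogue trigger in which a stolen-purse victim asks the player for help.
; On BeginPlay it creates a WB_Dialogue widget with the plea text.
; When BP_ThirdPersonCharacter overlaps the capsule, it shows the widget, switches to UI-only input, ignores movement and shows the cursor.
; AlreadyInteracted guards against repeat triggers until the character leaves the capsule; input is not restored here.
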(event OnComponentBeginOverlap(CapsuleComponent)
  (params (OverlappedComponent :type Primitive%20Component%20Object%20Reference) (OtherActor :type Actor%20Object%20Reference) (OtherComp :type Primitive%20Component%20Object%20Reference) (OtherBodyIndex :type Integer) (bFromSweep :type Boolean) (SweepResult :type Hit%20Result%20Structure%20%28by%20ref%29))
  (bind _asbp_third_person_character (Utilities|Casting|CastToBP_ThirdPersonCharacter OtherActor))
  (if (not (Variables|Default|GetAlreadyInteracted))
    (Variables|Default|SetAlreadyInteracted true)
    (UserInterface|Viewport|AddtoViewport (Variables|Default|GetDialogueBox) 0)
    (Input|SetInputModeUIOnly (Game|GetPlayerController (Variables|/Script/Engine.Pawn|GetPlayerState _asbp_third_person_character)) 0 "DoNotLock" false)
    (Input|SetIgnoreMoveInput (Game|GetPlayerController (Variables|/Script/Engine.Pawn|GetPlayerState _asbp_third_person_character)) true)
    (Variables|/Script/Engine.PlayerController|SetbShowMouseCursor (Game|GetPlayerController (Variables|/Script/Engine.Pawn|GetPlayerState _asbp_third_person_character)) true)))

(event OnComponentEndOverlap(CapsuleComponent)
  (params (OverlappedComponent :type Primitive%20Component%20Object%20Reference) (OtherActor :type Actor%20Object%20Reference) (OtherComp :type Primitive%20Component%20Object%20Reference) (OtherBodyIndex :type Integer))
  (Utilities|Casting|CastToBP_ThirdPersonCharacter OtherActor)
  (if (Variables|Default|GetAlreadyInteracted)
    (Variables|Default|SetAlreadyInteracted false)))

(event EventBeginPlay
  (bind _returnvalue (UserInterface|CreateWidget "/Game/SurvivalSemester/Level2/WB_Dialogue.WB_Dialogue_C"))
  (bind _output_get (Variables|Default|SetDialogueBox _returnvalue))
  (Variables|/Game/SurvivalSemester/Level2/WB_Dialogue.WB_Dialogue_C|SetTextDialogue _output_get "Someone stole my purse! 
Can you help me get it back?"))

(event Collision|EventActorBeginOverlap
  (params (OtherActor :type Actor%20Object%20Reference)))

(event EventTick
  (params (DeltaSeconds :type Float%20%28single-precision%29)))

(fn ConstructionScript)