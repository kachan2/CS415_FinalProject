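; BP_Seller is a vendor actor that shows a buy-item interface while the player character is near it.
; When BP_ThirdPersonCharacter enters InteractBox, it creates a WB_BuyItem widget, shows the mouse cursor and switches input to Game and UI, guarded by an InRadius flag against repeat triggers.
; Leaving the box removes the widget, hides the cursor and restores game-only input.
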(event OnComponentBeginOverlap(InteractBox)
  (params (OverlappedComponent :type Primitive%20Component%20Object%20Reference) (OtherActor :type Actor%20Object%20Reference) (OtherComp :type Primitive%20Component%20Object%20Reference) (OtherBodyIndex :type Integer) (bFromSweep :type Boolean) (SweepResult :type Hit%20Result%20Structure%20%28by%20ref%29))
  (bind _asbp_third_person_character (Utilities|Casting|CastToBP_ThirdPersonCharacter OtherActor))
  (if (not (Variables|Default|GetInRadius))
    (Variables|Default|SetInRadius true)
    (bind _returnvalue (UserInterface|CreateWidget "/Game/SurvivalSemester/UI/Widgets/WB_BuyItem.WB_BuyItem_C"))
    (bind _output_get (Variables|Default|SetBuyItemWidget _returnvalue))
    (UserInterface|Viewport|AddtoViewport _output_get 0)
    (Variables|/Script/Engine.PlayerController|SetbShowMouseCursor (Game|GetPlayerController (Variables|/Script/Engine.Pawn|GetPlayerState _asbp_third_person_character)) true)
    (Input|SetInputModeGameandUI (Game|GetPlayerController (Variables|/Script/Engine.Pawn|GetPlayerState _asbp_third_person_character)) 0 "DoNotLock" true false)))

(event OnComponentEndOverlap(InteractBox)
  (params (OverlappedComponent :type Primitive%20Component%20Object%20Reference) (OtherActor :type Actor%20Object%20Reference) (OtherComp :type Primitive%20Component%20Object%20Reference) (OtherBodyIndex :type Integer))
  (bind _asbp_third_person_character (Utilities|Casting|CastToBP_ThirdPersonCharacter OtherActor))
  (Variables|Default|SetInRadius false)
  (Widget|RemovefromParent (Variables|Default|GetBuyItemWidget))
  (Input|SetInputModeGameOnly (Game|GetPlayerController (Variables|/Script/Engine.Pawn|GetPlayerState _asbp_third_person_character)) false)
  (Variables|/Script/Engine.PlayerController|SetbShowMouseCursor (Game|GetPlayerController (Variables|/Script/Engine.Pawn|GetPlayerState _asbp_third_person_character)) false))

(fn ConstructionScript)