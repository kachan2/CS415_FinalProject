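; Trigger actor for the Level 3 dealer minigame, showing the WB_ThePriceIsRight widget when the third-person character enters its box.
; The widget is created at BeginPlay; on overlap, unless completed or already visible, it takes UI-only input, shows the cursor and blocks movement.
; Opening it pauses BP_Bus background sound and plays minigame audio; leaving the box swaps the audio back.
; Completion and input restoration are not handled here.
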(event OnComponentBeginOverlap(Box)
  (params (OverlappedComponent :type Primitive%20Component%20Object%20Reference) (OtherActor :type Actor%20Object%20Reference) (OtherComp :type Primitive%20Component%20Object%20Reference) (OtherBodyIndex :type Integer) (bFromSweep :type Boolean) (SweepResult :type Hit%20Result%20Structure%20%28by%20ref%29))
  (bind _gamewidget (Variables|Default|GetGameWidget))
  (bind _asbp_third_person_character (Utilities|Casting|CastToBP_ThirdPersonCharacter OtherActor))
  (if (not (Variables|Default|GetPlayerInRange?))
    (Variables|Default|SetPlayerInRange? true)
    (if (not (Variables|Default|GetCompletedMinigame?))
      (if (not (Widget|IsVisible _gamewidget))
        (UserInterface|Viewport|AddtoViewport _gamewidget 0)
        (Input|SetInputModeUIOnly (Game|GetPlayerController (Variables|/Script/Engine.Pawn|GetPlayerState _asbp_third_person_character)) 0 "DoNotLock" false)
        (Variables|/Script/Engine.PlayerController|SetbShowMouseCursor (Game|GetPlayerController (Variables|/Script/Engine.Pawn|GetPlayerState _asbp_third_person_character)) true)
        (Input|SetIgnoreMoveInput (Game|GetPlayerController (Variables|/Script/Engine.Pawn|GetPlayerState _asbp_third_person_character)) true)
        (bind _returnvalue (Actor|GetActorOfClass "/Game/SurvivalSemester/Level3/Blueprints/BP_Bus.BP_Bus_C"))
        (Class|AudioComponent|SetPaused (Variables|/Game/SurvivalSemester/Level3/Blueprints/BP_Bus.BP_Bus_C|GetBackgroundSound _returnvalue) true)
        (bind _returnvalue_2 (Audio|SpawnSound2D "/Game/SurvivalSemester/Level3/Level3Audio/level3minigameAudio.level3minigameAudio" 1.0 1.0 0.0 0))
        (Variables|Default|SetMiniGameSound _returnvalue_2)))))

(event OnComponentEndOverlap(Box)
  (params (OverlappedComponent :type Primitive%20Component%20Object%20Reference) (OtherActor :type Actor%20Object%20Reference) (OtherComp :type Primitive%20Component%20Object%20Reference) (OtherBodyIndex :type Integer))
  (Utilities|Casting|CastToBP_ThirdPersonCharacter OtherActor)
  (Variables|Default|SetPlayerInRange? false)
  (Class|AudioComponent|SetPaused (Variables|Default|GetMiniGameSound) true)
  (bind _returnvalue (Actor|GetActorOfClass "/Game/SurvivalSemester/Level3/Blueprints/BP_Bus.BP_Bus_C"))
  (Class|AudioComponent|SetPaused (Variables|/Game/SurvivalSemester/Level3/Blueprints/BP_Bus.BP_Bus_C|GetBackgroundSound _returnvalue) false))

(event EventBeginPlay
  (bind _returnvalue (UserInterface|CreateWidget "/Game/SurvivalSemester/Level3/Level3Minigame/WB_ThePriceIsRight.WB_ThePriceIsRight_C"))
  (Variables|Default|SetGameWidget _returnvalue))

(event Collision|EventActorBeginOverlap
  (params (OtherActor :type Actor%20Object%20Reference)))

(event EventTick
  (params (DeltaSeconds :type Float%20%28single-precision%29)))

(fn ConstructionScript)