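; BP_PetBowl is a pet bowl interactable that prompts the player to feed their dog.
; When the player character enters the Box, it opens a WB_CompleteTask widget for the "Dog" task, switches to UI-only input, ignores movement and shows the cursor.
; A PlayerInRange flag blocks repeat prompts until the character ends overlap with the StaticMesh, rather than the Box.
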(event OnComponentBeginOverlap(Box)
  (params (OverlappedComponent :type Primitive%20Component%20Object%20Reference) (OtherActor :type Actor%20Object%20Reference) (OtherComp :type Primitive%20Component%20Object%20Reference) (OtherBodyIndex :type Integer) (bFromSweep :type Boolean) (SweepResult :type Hit%20Result%20Structure%20%28by%20ref%29))
  (bind _asbp_third_person_character (Utilities|Casting|CastToBP_ThirdPersonCharacter OtherActor))
  (if (not (Variables|Default|GetPlayerInRange?))
    (Variables|Default|SetPlayerInRange? true)
    (bind _returnvalue (UserInterface|CreateWidget "/Game/SurvivalSemester/Level3/Widgets/WB_CompleteTask.WB_CompleteTask_C"))
    (Variables|/Game/SurvivalSemester/Level3/Widgets/WB_CompleteTask.WB_CompleteTask_C|SetTask _returnvalue "Dog")
    (Rendering|Components|TextRender|SetText (Variables|/Game/SurvivalSemester/Level3/Widgets/WB_CompleteTask.WB_CompleteTask_C|GetQuestionText _returnvalue) "Feed Your Dog?")
    (UserInterface|Viewport|AddtoViewport _returnvalue 0)
    (Input|SetInputModeUIOnly (Game|GetPlayerController (Variables|/Script/Engine.Pawn|GetPlayerState _asbp_third_person_character)) 0 "DoNotLock" false)
    (Input|SetIgnoreMoveInput (Game|GetPlayerController (Variables|/Script/Engine.Pawn|GetPlayerState _asbp_third_person_character)) true)
    (Variables|/Script/Engine.PlayerController|SetbShowMouseCursor (Game|GetPlayerController (Variables|/Script/Engine.Pawn|GetPlayerState _asbp_third_person_character)) true)))

(event OnComponentEndOverlap(StaticMesh)
  (params (OverlappedComponent :type Primitive%20Component%20Object%20Reference) (OtherActor :type Actor%20Object%20Reference) (OtherComp :type Primitive%20Component%20Object%20Reference) (OtherBodyIndex :type Integer))
  (Utilities|Casting|CastToBP_ThirdPersonCharacter OtherActor)
  (Variables|Default|SetPlayerInRange? false))

(event EventBeginPlay)

(event Collision|EventActorBeginOverlap
  (params (OtherActor :type Actor%20Object%20Reference)))

(fn ConstructionScript)