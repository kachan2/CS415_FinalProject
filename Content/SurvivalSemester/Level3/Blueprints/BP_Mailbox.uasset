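; BP_Mailbox is a Survival Semester Level 3 task object where the player is asked to drop off mail.
; It creates a task widget on BeginPlay and shows it when the third-person character enters its box, switching to UI-only input with a cursor and ignored movement.
; Tick polls TaskComplete, which is not set here, then once removes the message widget and starts a countdown widget for finding the bus.
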(event OnComponentBeginOverlap(Box)
  (params (OverlappedComponent :type Primitive%20Component%20Object%20Reference) (OtherActor :type Actor%20Object%20Reference) (OtherComp :type Primitive%20Component%20Object%20Reference) (OtherBodyIndex :type Integer) (bFromSweep :type Boolean) (SweepResult :type Hit%20Result%20Structure%20%28by%20ref%29))
  (bind _asbp_third_person_character (Utilities|Casting|CastToBP_ThirdPersonCharacter OtherActor))
  (if (not (Variables|Default|GetTaskComplete?))
    (if (not (Widget|IsVisible (Variables|Default|GetTaskWidget)))
      (UserInterface|Viewport|AddtoViewport (Variables|Default|GetTaskWidget) 0)
      (Input|SetInputModeUIOnly (Game|GetPlayerController (Variables|/Script/Engine.Pawn|GetPlayerState _asbp_third_person_character)) 0 "DoNotLock" false)
      (Input|SetIgnoreMoveInput (Game|GetPlayerController (Variables|/Script/Engine.Pawn|GetPlayerState _asbp_third_person_character)) true)
      (Variables|/Script/Engine.PlayerController|SetbShowMouseCursor (Game|GetPlayerController (Variables|/Script/Engine.Pawn|GetPlayerState _asbp_third_person_character)) true))))

(event OnComponentEndOverlap(Box)
  (params (OverlappedComponent :type Primitive%20Component%20Object%20Reference) (OtherActor :type Actor%20Object%20Reference) (OtherComp :type Primitive%20Component%20Object%20Reference) (OtherBodyIndex :type Integer))
  (Utilities|Casting|CastToBP_ThirdPersonCharacter OtherActor))

(event EventTick
  (params (DeltaSeconds :type Float%20%28single-precision%29))
  (if (Variables|Default|GetTaskComplete?)
    (if (not (Variables|Default|GetShowedNextTask))
      (Variables|Default|SetShowedNextTask true)
      (Widget|RemovefromParent (Variables|Default|GetMessageWidget))
      (bind _returnvalue (UserInterface|CreateWidget "/Game/SurvivalSemester/Level3/Widgets/WB_CountdownTimer.WB_CountdownTimer_C"))
      (Variables|/Game/SurvivalSemester/Level3/Widgets/WB_CountdownTimer.WB_CountdownTimer_C|SetMissionStatement _returnvalue "Find the bus before it leaves! ")
      (UserInterface|Viewport|AddtoViewport _returnvalue 0))))

(event EventBeginPlay
  (bind _returnvalue (UserInterface|CreateWidget "/Game/SurvivalSemester/Level3/Widgets/WB_CompleteTask.WB_CompleteTask_C"))
  (Variables|/Game/SurvivalSemester/Level3/Widgets/WB_CompleteTask.WB_CompleteTask_C|SetTask _returnvalue "Mailbox")
  (Rendering|Components|TextRender|SetText (Variables|/Game/SurvivalSemester/Level3/Widgets/WB_CompleteTask.WB_CompleteTask_C|GetQuestionText _returnvalue) "drop off mail?")
  (Variables|Default|SetTaskWidget _returnvalue))

(fn ConstructionScript)