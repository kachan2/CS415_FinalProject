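; BP_TaskCheckBox is a Level 3 trigger box that checks whether the player has completed the level's tasks.
; When the third-person character overlaps it, any incomplete entry in LevelTasks triggers a one-time game over, showing that task's ReasonOfDeath in a WB_GameOver widget with UI-only input and a mouse cursor.
; After the loop it prints a "FIND THE BUS!" message, whether or not the game ended.
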(event OnComponentBeginOverlap(Box)
  (params (OverlappedComponent :type Primitive%20Component%20Object%20Reference) (OtherActor :type Actor%20Object%20Reference) (OtherComp :type Primitive%20Component%20Object%20Reference) (OtherBodyIndex :type Integer) (bFromSweep :type Boolean) (SweepResult :type Hit%20Result%20Structure%20%28by%20ref%29))
  (bind _asbp_third_person_character (Utilities|Casting|CastToBP_ThirdPersonCharacter OtherActor))
  (for _array_element (Variables|Default|GetLevelTasks)
    (if (not (.Complete? (Utilities|Struct|BreakS_Tasks _array_element)))
      (if (not (Variables|/Game/ThirdPerson/Blueprints/BP_ThirdPersonCharacter.BP_ThirdPersonCharacter_C|GetGameOver? _asbp_third_person_character))
        (Variables|/Game/ThirdPerson/Blueprints/BP_ThirdPersonCharacter.BP_ThirdPersonCharacter_C|SetGameOver? _asbp_third_person_character true)
        (bind _returnvalue (UserInterface|CreateWidget "/Game/SurvivalSemester/UI/Widgets/WB_GameOver.WB_GameOver_C"))
        (Rendering|Components|TextRender|SetText (Variables|/Game/SurvivalSemester/UI/Widgets/WB_GameOver.WB_GameOver_C|GetTextBlock_0 _returnvalue) (.ReasonOfDeath (Utilities|Struct|BreakS_Tasks _array_element)))
        (UserInterface|Viewport|AddtoViewport _returnvalue 0)
        (Variables|/Script/Engine.PlayerController|SetbShowMouseCursor (Game|GetPlayerController (Variables|/Script/Engine.Pawn|GetPlayerState _asbp_third_person_character)) true)
        (Input|SetInputModeUIOnly (Game|GetPlayerController (Variables|/Script/Engine.Pawn|GetPlayerState _asbp_third_person_character)) _returnvalue "DoNotLock" false))))
  (Development|PrintString "FIND THE BUS!"))

(event EventBeginPlay)

(event Collision|EventActorBeginOverlap
  (params (OtherActor :type Actor%20Object%20Reference)))

(event EventTick
  (params (DeltaSeconds :type Float%20%28single-precision%29)))

(fn ConstructionScript)