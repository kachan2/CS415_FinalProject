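; BP_DecoyItems is a placeable decoy item in Level 3 that prompts the player with a question when approached.
; The construction script picks a decoy entry from an array by index and applies its mesh.
; When the third-person character enters the box, it shows a WB_DecoyTasks widget with the item's message, switches to UI-only input with a cursor and blocks movement.
; An in-range flag, cleared on exit, prevents repeat prompts.
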(event OnComponentBeginOverlap(Box)
  (params (OverlappedComponent :type Primitive%20Component%20Object%20Reference) (OtherActor :type Actor%20Object%20Reference) (OtherComp :type Primitive%20Component%20Object%20Reference) (OtherBodyIndex :type Integer) (bFromSweep :type Boolean) (SweepResult :type Hit%20Result%20Structure%20%28by%20ref%29))
  (bind _decoyitem (Variables|Default|GetDecoyItem))
  (bind _asbp_third_person_character (Utilities|Casting|CastToBP_ThirdPersonCharacter OtherActor))
  (if (not (Variables|Default|GetPlayerInRange?))
    (Variables|Default|SetPlayerInRange? true)
    (bind _returnvalue (UserInterface|CreateWidget "/Game/SurvivalSemester/Level3/Widgets/WB_DecoyTasks.WB_DecoyTasks_C"))
    (Variables|/Game/SurvivalSemester/Level3/Widgets/WB_DecoyTasks.WB_DecoyTasks_C|SetDecoyItemInQuestion _returnvalue _decoyitem)
    (Rendering|Components|TextRender|SetText (Variables|/Game/SurvivalSemester/Level3/Widgets/WB_DecoyTasks.WB_DecoyTasks_C|GetQuestionText _returnvalue) (Utilities|Text|ToText(String) (.MessageText (Utilities|Struct|BreakS_Decoys _decoyitem))))
    (UserInterface|Viewport|AddtoViewport _returnvalue 0)
    (Input|SetInputModeUIOnly (Game|GetPlayerController (Variables|/Script/Engine.Pawn|GetPlayerState _asbp_third_person_character)) 0 "DoNotLock" false)
    (Variables|/Script/Engine.PlayerController|SetbShowMouseCursor (Game|GetPlayerController (Variables|/Script/Engine.Pawn|GetPlayerState _asbp_third_person_character)) true)
    (Input|SetIgnoreMoveInput (Game|GetPlayerController (Variables|/Script/Engine.Pawn|GetPlayerState _asbp_third_person_character)) true)))

(event OnComponentEndOverlap(Box)
  (params (OverlappedComponent :type Primitive%20Component%20Object%20Reference) (OtherActor :type Actor%20Object%20Reference) (OtherComp :type Primitive%20Component%20Object%20Reference) (OtherBodyIndex :type Integer))
  (Utilities|Casting|CastToBP_ThirdPersonCharacter OtherActor)
  (Variables|Default|SetPlayerInRange? false))

(fn ConstructionScript
  (bind _output_get (Variables|Default|SetDecoyItem (Utilities|Array|Get(acopy) (Variables|Default|GetDecoyItems) (Variables|Default|GetItemIdx))))
  (Components|StaticMesh|SetStaticMesh (Variables|Default|GetStaticMesh) (.DecoyMesh (Utilities|Struct|BreakS_Decoys _output_get))))