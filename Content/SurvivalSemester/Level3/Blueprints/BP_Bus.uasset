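; BP_Bus is the level exit in Survival Semester's Level 3, ending the level when the player reaches it.
; When BP_ThirdPersonCharacter overlaps its Box, it sets the character's GameOver flag, which also blocks repeat triggers.
; It then shows the WB_NextLevel widget, ignores move input, switches to UI-only input and shows the mouse cursor.
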(event OnComponentBeginOverlap(Box)
  (params (OverlappedComponent :type Primitive%20Component%20Object%20Reference) (OtherActor :type Actor%20Object%20Reference) (OtherComp :type Primitive%20Component%20Object%20Reference) (OtherBodyIndex :type Integer) (bFromSweep :type Boolean) (SweepResult :type Hit%20Result%20Structure%20%28by%20ref%29))
  (bind _returnvalue (Game|GetPlayerState 0))
  (bind _returnvalue_2 (Game|GetPlayerController _returnvalue))
  (bind _asbp_third_person_character (Utilities|Casting|CastToBP_ThirdPersonCharacter OtherActor))
  (if (not (Variables|/Game/ThirdPerson/Blueprints/BP_ThirdPersonCharacter.BP_ThirdPersonCharacter_C|GetGameOver? _asbp_third_person_character))
    (Variables|/Game/ThirdPerson/Blueprints/BP_ThirdPersonCharacter.BP_ThirdPersonCharacter_C|SetGameOver? _asbp_third_person_character true)
    (bind _returnvalue_3 (UserInterface|CreateWidget "/Game/SurvivalSemester/UI/Widgets/WB_NextLevel.WB_NextLevel_C"))
    (UserInterface|Viewport|AddtoViewport _returnvalue_3 0)
    (Input|SetIgnoreMoveInput _returnvalue_2 true)
    (Input|SetInputModeUIOnly _returnvalue_2 0 "DoNotLock" false)
    (Variables|/Script/Engine.PlayerController|SetbShowMouseCursor _returnvalue_2 true)))

(event EventBeginPlay)

(event Collision|EventActorBeginOverlap
  (params (OtherActor :type Actor%20Object%20Reference)))

(event EventTick
  (params (DeltaSeconds :type Float%20%28single-precision%29)))

(fn ConstructionScript)