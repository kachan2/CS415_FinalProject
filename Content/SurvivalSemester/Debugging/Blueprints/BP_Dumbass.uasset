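; BP_Dumbass is a debugging actor with a health value that reacts to damage and destroys itself.
; Any damage received outside invincibility is added to Health, not subtracted, and the new value is printed.
; Each hit starts an invincibility window through a flag and a short Delay.
; Tick polls Health every frame and destroys the actor once it is zero or below.
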(event EventTick
  (params (DeltaSeconds :type Float%20%28single-precision%29))
  (if (<= (Variables|Default|GetHealth) 0.0)
    (Actor|DestroyActor)))

(event Game|Damage|EventAnyDamage
  (params (Damage :type Float%20%28single-precision%29) (DamageType :type Damage%20Type%20Object%20Reference) (InstigatedBy :type Controller%20Object%20Reference) (DamageCauser :type Actor%20Object%20Reference))
  (if (not (Variables|Default|GetIsInvincible))
    (Variables|Default|SetIsInvincible true)
    (bind _output_get (Variables|Default|SetHealth (+ (Variables|Default|GetHealth) Damage)))
    (Development|PrintString (Utilities|String|ToString(Float) _output_get))
    (Utilities|FlowControl|Delay 1.5)
    (Variables|Default|SetIsInvincible false)))

(fn ConstructionScript)